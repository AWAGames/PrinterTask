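; Window blind actor that opens and closes by rotating a set of static-mesh slats.
; On BeginPlay, OpenWindow plays a timeline that sets the slats straight to zero rotation, without interpolation.
; CloseWindos uses a second timeline to lerp them toward a tilted angle, starting from one slat's current rotation each update.
; Box overlap events are empty, leaving the widget and interaction-flag logic disconnected.
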(event OnComponentBeginOverlap(Box)
  (params (OverlappedComponent :type Primitive%20Component%20Object%20Reference) (OtherActor :type Actor%20Object%20Reference) (OtherComp :type Primitive%20Component%20Object%20Reference) (OtherBodyIndex :type Integer) (bFromSweep :type Boolean) (SweepResult :type Hit%20Result%20Structure%20%28by%20ref%29)))

(event OnComponentEndOverlap(Box)
  (params (OverlappedComponent :type Primitive%20Component%20Object%20Reference) (OtherActor :type Actor%20Object%20Reference) (OtherComp :type Primitive%20Component%20Object%20Reference) (OtherBodyIndex :type Integer)))

(event Custom|CloseWindos
  (bind _val (Timeline|Timeline_1 PlayFromStart)
    (:Update
      (Transformation|SetRelativeRotation (Variables|Default|GetStaticMesh9) (Math|Rotator|Lerp(Rotator) (Variables|/Script/Engine.SceneComponent|GetRelativeRotation (Variables|Default|GetStaticMesh5)) "-86.000000,0.000000, 0" _val) false false))))

(event Custom|OpenWindow
  (bind _val (Timeline|Timeline_0 PlayFromStart)
    (:Update
      (Transformation|SetRelativeRotation (Variables|Default|GetStaticMesh15) "0, 0, 0" false false))))

(event Custom|DoTask
  (params (Target :type Scene%20Component%20Object%20Reference) (NewRotation :type Rotator))
  (Transformation|SetRelativeRotation Target NewRotation false false))

(event EventBeginPlay
  (CallFunction|OpenWindow))

(fn ConstructionScript)