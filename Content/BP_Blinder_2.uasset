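; BP_Blinder_2 is a window blind actor that opens and closes by rotating a set of static mesh slats.
; CloseWindos runs a timeline that lerps the slats from StaticMesh5's current rotation toward a fixed closed angle, re-reading that rotation each update.
; OpenWindow also plays a timeline but snaps the slats to zero rotation, leaving its lerp unused.
; A separate DoTask event sets any target's relative rotation.
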(event Custom|CloseWindos
  (bind _val (Timeline|Timeline_1 PlayFromStart)
    (:Update
      (Transformation|SetRelativeRotation (Variables|Default|GetStaticMesh9) (Math|Rotator|Lerp(Rotator) (Variables|/Script/Engine.SceneComponent|GetRelativeRotation (Variables|Default|GetStaticMesh5)) "-86.000000,0.000000, 0" _val) false false))))

(event Custom|OpenWindow
  (bind _val (Timeline|Timeline_0 PlayFromStart)
    (:Update
      (Transformation|SetRelativeRotation (Variables|Default|GetStaticMesh15) "0, 0, 0" false false))))

(event Custom|DoTask
  (params (Target :type Scene%20Component%20Object%20Reference) (NewRotation :type Rotator))
  (Transformation|SetRelativeRotation Target NewRotation false false))

(event EventBeginPlay)

(fn ConstructionScript)